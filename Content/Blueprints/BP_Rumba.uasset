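; BP_Rumba is an interactable, apparently a closet door, that can bring in the CantonAI levels.
; On Interact it plays a door-opening sound at its location and asks the player controller to verify the last past message.
; If that check passes, it loads CantonAI and CantonAIArriba as level instances.
; The fade mentioned in its comment is not implemented in this graph.
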(event EventBeginPlay
  (|CallParentFunction) ; This node is disabled and will not be called.\nDrag off pins to build functionality.
)

(event Collision|EventActorBeginOverlap
  (params (OtherActor :type Actor%20Object%20Reference)))

(event EventTick
  (params (DeltaSeconds :type Float%20%28single-precision%29)))

(event EventInteract
  ;[0.15 0.15 0.15 0.5] Logica de sonido(Abrir puerte de closet) y difuminado
  (Audio|PlaySoundatLocation "/Game/Sound/audios/15419__pagancow__dorm-door-opening.15419__pagancow__dorm-door-opening" (Transformation|GetActorLocation) "0, 0, 0" 1.0 1.0 0.0 0 0 0 0)
  (bind _yes_ (Class|BPIVerifyObjects|VerifyLastPast(Message) (Game|GetPlayerController 0)))
  (if _yes_
    (Class|LevelStreamingDynamic|LoadLevelInstancebySoftObjectPtr "/Game/Dupy/level/CantonAI.CantonAI" "0, 0, 0" "0, 0, 0" "" 0 false)
    (Class|LevelStreamingDynamic|LoadLevelInstancebySoftObjectPtr "/Game/Dupy/level/cantonAIArriba.cantonAIArriba" "0, 0, 0" "0, 0, 0" "" 0 false)))

(fn ConstructionScript
  (|CallParentFunction))