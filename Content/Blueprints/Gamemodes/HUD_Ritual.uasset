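; Ritual game mode HUD that shows and closes the skill-check minigame widgets.
; Show switches on widget type, creating the Hilo or In and Out widget once and reusing it, with Hilo also receiving a skill-check count and starting a check.
; CloseSkill hides Hilo and ends In and Out if valid.
; The Knife fade is a placeholder print, with an unwired node intended to stop player movement.
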(event EventBeginPlay)

(event EventCloseSkill
  (Widget|SetVisibility (stale EventShow _returnvalue) "Hidden")
  (Utilities|IsValid (stale EventShow _returnvalue_2)
    (:Is%20Valid
      (Default|EndSkillCheck (stale EventShow _returnvalue_2)))))

(event EventShow
  (params (TypeOfWidget :type E_TypeOfWidget%20Enum :default "NewEnumerator0") (NumOfSkillCheck :type Integer))
  (switch Utilities|FlowControl|Switch|SwitchonE_TypeOfWidget TypeOfWidget
    (:NewEnumerator0
      (Utilities|FlowControl|Sequence
        (:then_0
          (Utilities|FlowControl|DoOnce false
            (:Completed
              (bind _returnvalue (UserInterface|CreateWidget "/Game/UI/WBP_HiloMinigame.WBP_HiloMinigame_C" (Game|GetPlayerController 0)))
              (UserInterface|Viewport|AddtoViewport _returnvalue 0))))
        (:then_1
          (Variables|/Game/UI/WBP_HiloMinigame.WBP_HiloMinigame_C|SetNumOISkillcheck _returnvalue NumOfSkillCheck)
          (Widget|SetVisibility _returnvalue "Visible")
          (Default|NewSkillCheck _returnvalue))))
    (:NewEnumerator1
      (Utilities|FlowControl|Sequence
        (:then_0
          (Utilities|FlowControl|DoOnce false
            (:Completed
              (bind _returnvalue_2 (UserInterface|CreateWidget "/Game/UI/WBP_InAndOutMinigame.WBP_InAndOutMinigame_C" (Game|GetPlayerController 0)))
              (UserInterface|Viewport|AddtoViewport _returnvalue_2 0))))
        (:then_1
          (Widget|SetVisibility _returnvalue_2 "Visible"))))
    (:NewEnumerator2
      ;[0.15 0.15 0.15 0.5] Aqui voy a poner la logica del difuminado
      (Development|PrintString "Difuminado"))))

(fn ConstructionScript)