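; Interactable plush teddy for a ritual, advanced through cutting, stuffing, threading and pickup by an Objective state switch.
; Interact checks the knife and box via the player controller, creates its message widgets, plays step sounds and updates HUD_Ritual's instructions in some steps.
; Stuffing passes a skill-check count; a separate Terminated event unlocks threading after a timer.
; The final interaction points the player to filling the bathtub and destroys the actor.
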(event Custom|NextEvent
  (Class|BPIControlMovementPlayer|ControlMove(Message) (Game|Player|GetPlayerPawn 0))
  (Variables|Default|SetObjective "NewEnumerator0")
  (Rendering|SetVisibility (Variables|Default|GetWidget) true false))

(event EventBeginPlay
  (|CallParentFunction) ; This node is disabled and will not be called.\nDrag off pins to build functionality.
)

(event EventTerminated
  (bind _ashud_ritual (Utilities|Casting|CastToHUD_Ritual (HUD|GetHUD (Game|GetPlayerController 0))))
  (Default|UpdateRitualStep (Variables|/Game/Blueprints/Gamemodes/HUD_Ritual.HUD_Ritual_C|GetRitualStepsWidget _ashud_ritual) "Agarra el muñeco otra vez")
  (Utilities|Time|SetTimerbyEvent (delegate Custom|NextEvent) 5.0))

(event EventInteract
  (bind _returnvalue (Game|GetPlayerController 0))
  (switch Utilities|FlowControl|Switch|SwitchonE_TypeOfWidget (Variables|Default|GetObjective)
    (:NewEnumerator0
      ;[0.15 0.15 0.15 0.5] Misma logica de difunidad y sonido(Enredar al peluche en cordon)
      (Class|BPICreateWidgets|Create(Message) _returnvalue "NewEnumerator2")
      (Audio|PlaySoundatLocation "/Game/Sound/audios/649926__samram21__knitting-needles.649926__samram21__knitting-needles" (Transformation|GetActorLocation) "0, 0, 0" 1.0 1.0 0.0 0 0 0 0)
      (Variables|Default|SetObjective "NewEnumerator3")
      (Class|BPIPlayerGetObjects|GetPlush(Message) (Game|GetPlayerController 0)))
    (:NewEnumerator1
      ;[0.15 0.15 0.15 0.5] Logica de sonido(tirar cosas de una caja)
      (bind _hasbox_ (Class|BPIVerifyObjects|VerifyBox(Message) _returnvalue))
      (if _hasbox_
        (Audio|PlaySoundatLocation "/Game/Sound/audios/364735__newagesoup__foley-handle-cardboard-box.364735__newagesoup__foley-handle-cardboard-box" (Transformation|GetActorLocation) "0, 0, 0" 1.0 1.0 0.0 0 0 0 0)
        (Class|BPICreateWidgets|Create(Message) _returnvalue (Variables|Default|GetObjective) (Variables|Default|GetNumOfSkillCheck))
        (Rendering|SetVisibility (Variables|Default|GetWidget) false false)))
    (:NewEnumerator2
      (bind _ashud_ritual (Utilities|Casting|CastToHUD_Ritual (HUD|GetHUD (Game|GetPlayerController 0))))
      (Default|UpdateRitualStep (Variables|/Game/Blueprints/Gamemodes/HUD_Ritual.HUD_Ritual_C|GetRitualStepsWidget _ashud_ritual) "Rellena el muñeco")
      (bind _hasknife (Class|BPIVerifyObjects|Verifyknife(Message) _returnvalue))
      (if _hasknife
        ;[0.15 0.15 0.15 0.5] Aqui va la logica de difuminado y del sonido de rasgado
        (Audio|PlaySoundatLocation "/Game/Sound/audios/817731__spinopel__torn-paper.817731__spinopel__torn-paper" (Transformation|GetActorLocation) "0, 0, 0" 1.0 1.0 0.0 0 0 0 0)
        (Class|BPICreateWidgets|Create(Message) _returnvalue "NewEnumerator2")
        (Variables|Default|SetObjective "NewEnumerator1")
        (else
          (bind _ashud_ritual_2 (Utilities|Casting|CastToHUD_Ritual (HUD|GetHUD (Game|GetPlayerController 0))))
          (Default|UpdateRitualStep (Variables|/Game/Blueprints/Gamemodes/HUD_Ritual.HUD_Ritual_C|GetRitualStepsWidget _ashud_ritual_2) "Agarra el cuchillo e intenta de nuevo"))))
    (:NewEnumerator3
      (bind _ashud_ritual_3 (Utilities|Casting|CastToHUD_Ritual (HUD|GetHUD (Game|GetPlayerController 0))))
      ;[0.15 0.15 0.15 0.5] Aqui por si se ocupa mover
      (Default|UpdateRitualStep (Variables|/Game/Blueprints/Gamemodes/HUD_Ritual.HUD_Ritual_C|GetRitualStepsWidget _ashud_ritual_3) "Agarra el agua y llena la bañera")
      ;;[0.15 0.15 0.15 0.5] Logica de decir el nombre y decidirle el nombre para que despues inmediatamente lo agarre(Sonido de agarrar)
      (Audio|PlaySoundatLocation "/Game/Sound/audios/188431__qubodup__epic-object-placing.188431__qubodup__epic-object-placing" (Transformation|GetActorLocation) "0, 0, 0" 1.0 1.0 0.0 0 0 0 0)
      (Actor|DestroyActor))))

(fn ConstructionScript
  (|CallParentFunction))