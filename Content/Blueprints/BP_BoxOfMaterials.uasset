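; BP_BoxOfMaterials is an interactable box of materials that advances the ritual objective when picked up.
; On Interact, it gets HUD_Ritual from the player controller and sets the ritual step text, in Spanish, to find a plush toy and stab it.
; It then plays a cardboard box sound at its location, calls GetBoxMessage on the player controller and destroys itself.
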(event EventBeginPlay
  (|CallParentFunction) ; This node is disabled and will not be called.\nDrag off pins to build functionality.
)

(event Collision|EventActorBeginOverlap
  (params (OtherActor :type Actor%20Object%20Reference)))

(event EventTick
  (params (DeltaSeconds :type Float%20%28single-precision%29)))

(event EventInteract
  (bind _ashud_ritual (Utilities|Casting|CastToHUD_Ritual (HUD|GetHUD (Game|GetPlayerController 0))))
  (Default|UpdateRitualStep (Variables|/Game/Blueprints/Gamemodes/HUD_Ritual.HUD_Ritual_C|GetRitualStepsWidget _ashud_ritual) "Encuentra un peluche y acuchillalo")
  ;[0.15 0.15 0.15 0.5] Logica de sonido (Agarrar caja de muchas cosas)
  (Audio|PlaySoundatLocation "/Game/Sound/audios/364735__newagesoup__foley-handle-cardboard-box.364735__newagesoup__foley-handle-cardboard-box" (Transformation|GetActorLocation) "0, 0, 0" 1.0 1.0 0.0 0 0 0 0)
  (Class|BPIPlayerGetObjects|GetBox(Message) (Game|GetPlayerController 0))
  (Actor|DestroyActor))

(fn ConstructionScript
  (|CallParentFunction))