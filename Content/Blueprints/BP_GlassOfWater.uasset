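; Interactable glass-of-water pickup that advances the ritual when the player uses it.
; Interact casts the player's HUD to HUD_Ritual and updates its steps widget with the hardcoded Spanish bathtub-and-doll objective.
; It then plays a pouring sound at its location, triggers message calls on the player controller and destroys itself.
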(event EventBeginPlay
  (|CallParentFunction) ; This node is disabled and will not be called.\nDrag off pins to build functionality.
)

(event EventInteract
  (bind _returnvalue (Game|GetPlayerController 0))
  (bind _ashud_ritual (Utilities|Casting|CastToHUD_Ritual (HUD|GetHUD (Game|GetPlayerController 0))))
  (Default|UpdateRitualStep (Variables|/Game/Blueprints/Gamemodes/HUD_Ritual.HUD_Ritual_C|GetRitualStepsWidget _ashud_ritual) "Llena la bañera y mete al muñeco al agua")
  ;[0.15 0.15 0.15 0.5] logica de sonido(Rellenar vaso de agua) y difuminado
  (Audio|PlaySoundatLocation "/Game/Sound/audios/163732__mrbriandesign__pouring-water-long.163732__mrbriandesign__pouring-water-long" (Transformation|GetActorLocation) "0, 0, 0" 1.0 1.0 0.0 0 0 0 0)
  (Class|BPICreateWidgets|Create(Message) _returnvalue "NewEnumerator2")
  (Class|BPIPlayerGetObjects|GetGlassOfWater(Message) _returnvalue)
  (Actor|DestroyActor))

(fn ConstructionScript
  (|CallParentFunction))