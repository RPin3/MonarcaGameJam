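; Knife pickup actor for the ritual sequence, collected through its Interact event.
; On Interact it casts the player's HUD to HUD_Ritual and sets the ritual step text to a Spanish prompt to go for the box of objects.
; It then plays a knife slash sound at its location, sends GetKnifeMessage to the player controller and destroys itself.
; If the HUD cast fails, nothing happens.
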(event EventBeginPlay
  (|CallParentFunction) ; This node is disabled and will not be called.\nDrag off pins to build functionality.
)

(event Collision|EventActorBeginOverlap
  (params (OtherActor :type Actor%20Object%20Reference)))

(event EventTick
  (params (DeltaSeconds :type Float%20%28single-precision%29)))

(event EventInteract
  (bind _ashud_ritual (Utilities|Casting|CastToHUD_Ritual (HUD|GetHUD (Game|GetPlayerController 0))))
  (Default|UpdateRitualStep (Variables|/Game/Blueprints/Gamemodes/HUD_Ritual.HUD_Ritual_C|GetRitualStepsWidget _ashud_ritual) "Ve por la caja con objetos")
  ;[0.15 0.15 0.15 0.5] logica de sonido, agarrra cuchillo
  (Audio|PlaySoundatLocation "/Game/Sound/audios/118792__lmbubec__1_knife_slash_a.118792__lmbubec__1_knife_slash_a" (Transformation|GetActorLocation) "0, 0, 0" 1.0 1.0 0.0 0 0 0 0)
  (Class|BPIPlayerGetObjects|GetKnife(Message) (Game|GetPlayerController 0))
  (Actor|DestroyActor))

(fn ConstructionScript
  (|CallParentFunction))