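; BP_Batuv is the interactable bathtub that drives steps of a plush-doll ritual.
; Each Interact runs a sequence: a one-shot gate fills the tub, another places the plush and opens a name-entry widget once the controller verifies it.
; With plush and TV confirmed, DoOnce branches update HUD objectives, then pause player control for timed subtitles, a knife slash and the hide prompt.
; State checks and notifications go through player controller and pawn messages.
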(event Custom|Move
  (Class|BPIControlMovementPlayer|ControlMove(Message) (Game|Player|GetPlayerPawn 0)))

(event EventBeginPlay
  (|CallParentFunction) ; This node is disabled and will not be called.\nDrag off pins to build functionality.
)

(event Collision|EventActorBeginOverlap
  (params (OtherActor :type Actor%20Object%20Reference)))

(event EventTick
  (params (DeltaSeconds :type Float%20%28single-precision%29)))

(event EventInteract
  (bind _returnvalue (Game|GetPlayerController 0))
  (bind _returnvalue_2 (Game|GetPlayerController 0))
  (bind _returnvalue_3 (Game|GetPlayerController 0))
  (bind _returnvalue_4 (Game|GetPlayerController 0))
  (Utilities|FlowControl|Sequence
    (:then_0
      (Utilities|FlowControl|Gate false :!label _label
        (:Exit
          ;[0.15 0.15 0.15 0.5] Logica de difuminado
          (Class|BPICreateWidgets|Create(Message) _returnvalue "NewEnumerator2")
          ;[0.15 0.15 0.15 0.5] Aqui va la logica de sonido(Rellenar tina de agua)
          (Audio|PlaySoundatLocation "/Game/Sound/audios/256869__hanstimm__water004ed.256869__hanstimm__water004ed" (Transformation|GetActorLocation) "0, 0, 0" 1.0 1.0 0.0 0 0 0 0)
          (Class|BPIPlayerGetObjects|GetBatuv(Message) _returnvalue)
          (goto _label Close))))
    (:then_1
      (Utilities|FlowControl|Gate false :!label _label_2
        (:Exit
          (bind _hasplush (Class|BPIVerifyObjects|VerifyPlush(Message) _returnvalue_3))
          (if _hasplush
            (Audio|PlaySoundatLocation "/Game/Sound/audios/188431__qubodup__epic-object-placing.188431__qubodup__epic-object-placing" (Transformation|GetActorLocation) "0, 0, 0" 1.0 1.0 0.0 0 0 0 0)
            ;[0.15 0.15 0.15 0.5] Difuminado
            (Class|BPICreateWidgets|Create(Message) _returnvalue_3 "NewEnumerator2")
            (Development|SetHiddeninGame (Variables|Default|GetPlush) false false)
            (Class|BPIVerifyObjects|VerifyPlushinPosition(Message) _returnvalue_3)
            (Variables|/Script/Engine.PlayerController|SetbShowMouseCursor _returnvalue_2 true)
            (bind _returnvalue_5 (UserInterface|CreateWidget "/Game/UI/Objectives/WBP_EnterName.WBP_EnterName_C" _returnvalue_2))
            (Input|SetInputModeUIOnly _returnvalue_2 _returnvalue_5 "DoNotLock" false)
            (UserInterface|Viewport|AddtoViewport _returnvalue_5 0)
            (goto _label_2 Close)))))
    (:then_2
      (bind _yes_ (Class|BPIPlayerGetObjects|PlushinPosition?(Message) _returnvalue_4))
      (if _yes_
        (Utilities|FlowControl|Sequence
          (:then_0
            (Utilities|FlowControl|DoOnce false
              (:Completed
                (bind _ashud_ritual (Utilities|Casting|CastToHUD_Ritual (HUD|GetHUD (Game|GetPlayerController 0))))
                (Default|UpdateRitualStep (Variables|/Game/Blueprints/Gamemodes/HUD_Ritual.HUD_Ritual_C|GetRitualStepsWidget _ashud_ritual) "Apaga el foco y prende la tele"))))
          (:then_1
            (bind _yes__2 (Class|BPIVerifyObjects|VerifyTvOn?(Message) _returnvalue_4))
            (if _yes__2
              (Utilities|FlowControl|DoOnce false
                (:Completed
                  (Class|BPIControlMovementPlayer|ControlStop(Message) (Game|Player|GetPlayerPawn 0))
                  (bind _returnvalue_6 (UserInterface|CreateWidget "/Game/UI/WBP_Subtitles.WBP_Subtitles_C" (Game|GetPlayerController 0)))
                  (bind _output_get (Variables|Default|SetWidget1 _returnvalue_6))
                  (Default|MostrarSubtitulo _returnvalue_6 "Linea_1")
                  (UserInterface|Viewport|AddtoViewport _returnvalue_6 0)
                  (Utilities|Time|SetTimerbyEvent (EventDispatchers|CreateEvent :!event Custom|Move) 6.0)
                  (Utilities|FlowControl|Delay 3.0)
                  ;[0.15 0.15 0.15 0.5] difuminado y aqui se puede poner el sonido del cuchillo
                  (Utilities|IsValid (Variables|Default|GetWidget1)
                    (:Is%20Valid
                      (Default|MostrarSubtitulo (Variables|Default|GetWidget1) "Linea_2")
                      (Utilities|FlowControl|Delay 3.0)
                      (Default|MostrarSubtitulo (Variables|Default|GetWidget1) "Linea_3"))
                    (:Is%20Not%20Valid
                      (bind _returnvalue_7 (UserInterface|CreateWidget "/Game/UI/WBP_Subtitles.WBP_Subtitles_C" (Game|GetPlayerController 0)))
                      (Default|MostrarSubtitulo _returnvalue_7 "Linea_2")
                      (UserInterface|Viewport|AddtoViewport _returnvalue_7 0)
                      (Utilities|FlowControl|Delay 3.0)
                      (Default|MostrarSubtitulo _returnvalue_7 "Linea_3")
                      (Widget|RemovefromParent _returnvalue_7)))
                  (Audio|PlaySoundatLocation "/Game/Sound/audios/118792__lmbubec__1_knife_slash_a.118792__lmbubec__1_knife_slash_a" (Transformation|GetActorLocation) "0, 0, 0" 1.0 1.0 0.0 0 0 0 0)
                  (bind _ashud_ritual_2 (Utilities|Casting|CastToHUD_Ritual (HUD|GetHUD (Game|GetPlayerController 0))))
                  ;[0.15 0.15 0.15 0.5] Cambiar escondite por lo que sea que sea el rumba
                  (Default|UpdateRitualStep (Variables|/Game/Blueprints/Gamemodes/HUD_Ritual.HUD_Ritual_C|GetRitualStepsWidget _ashud_ritual_2) "Corre al escondite")
                  (Input|SetInputModeGameOnly (Game|GetPlayerController 0) false)
                  (Class|BPICreateWidgets|Create(Message) (Game|GetPlayerController 0) "NewEnumerator2")
                  (Transformation|SetRelativeLocation (Variables|Default|GetPlush) "110.000000,0.000000,-50.000000" false false)
                  (Class|BPIPlayerGetObjects|LastPast(Message) (Game|GetPlayerController 0)))))))))))

(fn ConstructionScript
  (|CallParentFunction))