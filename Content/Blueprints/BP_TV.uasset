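; BP_TV is an interactable television that advances the ritual sequence.
; Interact, gated by the controller's all-switches-off check, runs once: it plays TV audio, shows a subtitle, and halts player control during a delay.
; It then restores movement and updates the HUD ritual step to stabbing the plush in the bathroom.
; PawnSensing feeds the MPC_TV "Enemy" parameter with the dot product of BP_IA and TV world locations.
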(event OnSeePawn(PawnSensing)
  (params (Pawn :type Pawn%20Object%20Reference))
  ;[0.15 0.15 0.15 0.5] aqui cambiar los valores del parameter
  (bind _asbp_ia (Utilities|Casting|CastToBP_IA Pawn))
  (Rendering|Material|SetScalarParameterValue "/Game/Materials/WorldShaders/TVShaders/MPC_TV.MPC_TV" "Enemy" (Math|Vector|DotProduct (Transformation|GetActorLocation _asbp_ia) (Transformation|GetActorLocation)) :!class /Script/Engine.KismetMaterialLibrary))

(event EventBeginPlay
  (|CallParentFunction) ; This node is disabled and will not be called.\nDrag off pins to build functionality.
)

(event Collision|EventActorBeginOverlap
  (params (OtherActor :type Actor%20Object%20Reference)))

(event EventTick
  (params (DeltaSeconds :type Float%20%28single-precision%29)))

(event EventInteract
  (bind _returnvalue (Game|Player|GetPlayerPawn 0))
  ;[0.15 0.15 0.15 0.5] Logica de sonido(Prender televisor y estatica) y el shader
  (bind _yes_ (Class|BPIVerifyObjects|VerifyAllSwitchOff(Message) (Game|GetPlayerController 0)))
  (if _yes_
    (Utilities|FlowControl|DoOnce false
      (:Completed
        (Audio|PlaySoundatLocation "/Game/Sound/audios/tv.tv" (Transformation|GetActorLocation) "0, 0, 0" 1.0 1.0 0.0 0 0 0 0)
        (Class|BPIPlayerGetObjects|Tvon(Message) (Game|GetPlayerController 0))
        (bind _returnvalue_2 (UserInterface|CreateWidget "/Game/UI/WBP_Subtitles.WBP_Subtitles_C"))
        (Default|MostrarSubtitulo _returnvalue_2 "Linea_4")
        (UserInterface|Viewport|AddtoViewport _returnvalue_2 0)
        (Class|BPIControlMovementPlayer|ControlStop(Message) _returnvalue)
        (Utilities|FlowControl|Delay 1e+01)
        (Class|BPIControlMovementPlayer|ControlMove(Message) _returnvalue)
        (bind _ashud_ritual (Utilities|Casting|CastToHUD_Ritual (HUD|GetHUD (Game|GetPlayerController 0))))
        (Default|UpdateRitualStep (Variables|/Game/Blueprints/Gamemodes/HUD_Ritual.HUD_Ritual_C|GetRitualStepsWidget _ashud_ritual) "Ve al baño y acuchilla al peluche")))))

(fn ConstructionScript
  (|CallParentFunction))