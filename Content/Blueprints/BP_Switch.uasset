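; BP_Switch is an interactable light switch that turns off its SpotLight.
; On Interact, a DoOnce gate plays the Turn_off sound at the actor's location, sets the light's intensity to zero and calls SwitchOffAddMessage on player controller 0.
; The gate is never reset, so the switch works only once and cannot turn the light back on.
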(event EventBeginPlay
  (|CallParentFunction) ; This node is disabled and will not be called.\nDrag off pins to build functionality.
)

(event Collision|EventActorBeginOverlap
  (params (OtherActor :type Actor%20Object%20Reference)))

(event EventTick
  (params (DeltaSeconds :type Float%20%28single-precision%29)))

(event EventInteract
  ;[0.15 0.15 0.15 0.5] Aqui se puede poner la logica de sonido(apagador de luz)
  (Utilities|FlowControl|DoOnce false
    (:Completed
      (Audio|PlaySoundatLocation "/Game/Sound/audios/turn_off.turn_off" (Transformation|GetActorLocation) "0, 0, 0" 1.0 1.0 0.0 0 0 0 0)
      (Rendering|Components|Light|SetIntensity (Variables|Default|GetSpotLight) 0.0)
      (Class|BPIPlayerGetObjects|SwitchOffAdd(Message) (Game|GetPlayerController 0)))))

(fn ConstructionScript
  (|CallParentFunction))